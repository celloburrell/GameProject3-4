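; Game mode that runs an elapsed-time clock for the level and returns to the MainMenu level on game over.
; BeginPlay creates the WBP_Timer widget and adds it to the viewport.
; Tick uses a one-second Delay to throttle counting of seconds, rolling over into minutes at 60.
; The GameOver event handles the level change.
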(event Custom|GameOver
  (Game|OpenLevel(byName) "MainMenu"))

(event EventBeginPlay
  (bind _returnvalue (UserInterface|CreateWidget "/Game/Project3/WBP_Timer.WBP_Timer_C"))
  (UserInterface|Viewport|AddtoViewport _returnvalue 0))

(event EventTick
  (params (DeltaSeconds :type Float%20%28single-precision%29))
  (Utilities|FlowControl|Delay 1.0)
  (Class|MyGameModeBase|IncrementTimeSeconds)
  (if (>= (Class|MyGameModeBase|GetTimeSeconds) 60)
    (Class|MyGameModeBase|IncrementTimeMinutes)
    (Class|MyGameModeBase|SetTimeSeconds)))

(fn ConstructionScript)